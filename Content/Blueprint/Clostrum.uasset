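; Clostrum sets up asymmetric local multiplayer at BeginPlay, spawning an Investigator and Dr. Zurk from the level's PlayerStarts.
; It loops over every PlayerStart, calling CreatePlayer with the array index, and adds IMC_Default to each player's Enhanced Input.
; Index 0 possesses a first-person character as the Investigator; higher indices possess third-person characters as Dr. Zurk.
; Roles and spawn points therefore depend on the order GetAllActorsOfClass returns.
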(event `self.ReceiveBeginPlay`
  (bind _returnvalue (`GameplayStatics.GetPlayerController` 0))
  ; pour chaque Player spawn
  (bind _outactors (`GameplayStatics.GetAllActorsOfClass` "/Script/Engine.PlayerStart"))
  (for (_array_element _array_index) _outactors
    (bind _output_get (set `self.Array Index` _array_index))
    (bind _returnvalue_2 (`GameplayStatics.CreatePlayer` _output_get))
    ; Dr.Zurk player
    (if (> (`self.Array Index`) 0)
      (`EnhancedInputSubsystemInterface.AddMappingContext` (pcsubsystem `EnhancedInputLocalPlayerSubsystem` _returnvalue_2) "/Game/ThirdPerson/Input/IMC_Default.IMC_Default" 0 (struct))
      (bind _returnvalue_3 (`self.GetTransform` _array_element))
      (bind _returnvalue_4 (`|SpawnActorFromClass` "/Game/ThirdPerson/Blueprints/BP_ThirdPersonCharacter.BP_ThirdPersonCharacter_C" _returnvalue_3 "Undefined" "MultiplyWithRoot" null null))
      (`Controller.Possess` (`GameplayStatics.GetPlayerController` (`self.Array Index`)) _returnvalue_4)
      (else
        ; Investigateur Player
        (`EnhancedInputSubsystemInterface.AddMappingContext` (pcsubsystem `EnhancedInputLocalPlayerSubsystem` _returnvalue) "/Game/FirstPerson/Input/IMC_Default.IMC_Default" 0 (struct))
        (bind _returnvalue_5 (`|SpawnActorFromClass` "/Game/FirstPerson/Blueprints/BP_FirstPersonCharacter.BP_FirstPersonCharacter_C" _returnvalue_3 "Undefined" "MultiplyWithRoot" null null))
        (`Controller.Possess` _returnvalue _returnvalue_5)))))

(fn `UserConstructionScript`)